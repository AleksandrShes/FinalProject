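; BP_Enemy1 is an AI enemy character Blueprint, largely at a debug stage.
; On BeginPlay it prints a greeting, sets its walk speed and calls OnHealthChange on its HealthComponent with zero.
; When AIPerception updates a target, it casts to Main_Char_BP and prints a hostile message if the TeamTag differs, or a friend message if the cast fails.
; The other perception events do nothing.
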(event `self.ReceiveBeginPlay`
  (`KismetSystemLibrary.PrintString` "HELLLLLLLLLLOOO!!!")
  (set `CharacterMovementComponent.MaxWalkSpeed` 400.0 (`self.CharacterMovement`))
  (`/Game/MyUI/Components/HealthComponent.OnHealthChange` (`self.HealthComponent`) 0.0))

(event `self.AIPerception.OnPerceptionUpdated`
  (params (UpdatedActors :type "Array of Actor Object Reference (by ref)")))

(event `self.AIPerception.OnTargetPerceptionForgotten`
  (params (Actor :type "Actor Object Reference")))

(event `self.AIPerception.OnTargetPerceptionUpdated`
  (params (Actor :type "Actor Object Reference") (Stimulus :type "AIStimulus Structure"))
  (bind _asmain_char_bp (cast `/Game/MyBlueprints/Main_Char_BP` Actor)
    (:`then`
      (if (!= (`/Game/MyBlueprints/Main_Char_BP.TeamTag` _asmain_char_bp) (`self.TeamTag`))
        (`KismetSystemLibrary.PrintString` "I Kill You")))
    (:`CastFailed`
      (`KismetSystemLibrary.PrintString` "FRIEND!"))))

(event `self.AIPerception.OnTargetPerceptionInfoUpdated`
  (params (UpdateInfo :type "ActorPerceptionUpdateInfo Structure (by ref)")))

(fn `UserConstructionScript`)