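; BP_AmmoBox_2 is an ammo pickup that passes its amount to the player's weapon Reload on overlap, then destroys itself.
; The construction script randomizes the amount, and BeginPlay shows it on a WBP_Ammo widget component.
; Tick shows the widget only when the camera is within a 2D range, running a Timeline that spins the mesh and turns the widget toward the camera, and stops it otherwise.
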(event `self.ReceiveTick`
  (params (DeltaSeconds :type "Float (single-precision)"))
  (bind _returnvalue (`GameplayStatics.GetPlayerCameraManager` 0))
  (bind _count (`self.Count`))
  (bind _count_2 (`self.Count`))
  (bind _returnvalue_2 (`SceneComponent.K2_GetComponentLocation` _count_2))
  ;[0 0 1] 3. Поворот виджета патронов
  ;[0 0 1] 4. Видимость виджета от расстояния до игрока
  (if (< (`KismetMathLibrary.Vector_Distance2D` _returnvalue_2 (`SceneComponent.K2_GetComponentLocation` (`Actor.RootComponent` _returnvalue))) 1500.0)
    (`SceneComponent.SetHiddenInGame` _count false false)
    ;[0 0 1] 5. Поворот магазина
    (bind (_direction _newtrack_0) (`Timeline|Timeline` :!label _label)
      (:`Update`
        (`SceneComponent.K2_SetRelativeRotation` (`self.StaticMeshComponent`) (`KismetMathLibrary.MakeRotator` 0.0 0.0 (* _newtrack_0 360.0)) false false)
        (`SceneComponent.K2_SetWorldRotation` _count_2 (`KismetMathLibrary.FindLookAtRotation` _returnvalue_2 (`SceneComponent.K2_GetComponentLocation` (`PlayerCameraManager.TransformComponent` _returnvalue))) false false)))
    (else
      (`SceneComponent.SetHiddenInGame` _count true false)
      (goto _label :!via `Stop`))))

(event `self.ReceiveBeginPlay`
  ;[1 1 1] Call Wiget AmmoCount
  (bind _aswbp_ammo (cast `/Game/MyUI/WBP_Ammo` (`WidgetComponent.GetUserWidgetObject` (`self.Count`))))
  (`/Game/MyUI/WBP_Ammo.SetAmmoCount` _aswbp_ammo (`self.AmmoAmount`)))

(event `self.Collision.OnComponentBeginOverlap`
  (params (OverlappedComponent :type "PrimitiveComponent Object Reference") (OtherActor :type "Actor Object Reference") (OtherComp :type "PrimitiveComponent Object Reference") (OtherBodyIndex :type Integer) (bFromSweep :type Boolean) (SweepResult :type "HitResult Structure (by ref)"))
  (bind _returnvalue (`GameplayStatics.GetPlayerCharacter` 0))
  (if (== OtherActor _returnvalue)
    (bind _asmain_char_bp (cast `/Game/MyBlueprints/Main_Char_BP` _returnvalue))
    (`/Game/MyBlueprints/Ka47_BP.Reload` (`/Game/MyBlueprints/Main_Char_BP.weapon` _asmain_char_bp) (`self.AmmoAmount`))
    (`self.K2_DestroyActor`)))

(fn `UserConstructionScript`
  (set `self.AmmoAmount` (`KismetMathLibrary.RandomIntegerInRange` 20 30)))