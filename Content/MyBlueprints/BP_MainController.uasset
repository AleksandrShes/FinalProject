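; BP_MainController is the player controller, handling health and death for the player character.
; AnyDamage feeds its HealthComponent, with debug keys 3 and 4 applying damage and negative damage to the controller itself.
; On death it disables character input, shows the cursor, pulls the camera back and up, and plays the death montage on both character meshes.
; The second montage's blend-out triggers a short delay, then quits the game.
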(event `self.ReceiveAnyDamage`
  (params (Damage :type "Float (single-precision)") (DamageType :type "DamageType Object Reference") (InstigatedBy :type "Controller Object Reference") (DamageCauser :type "Actor Object Reference"))
  (`/Game/MyUI/Components/HealthComponent.OnHealthChange` (`self.HealthComponent`) Damage))

(event `Key|Three`
  (params (Key :type "Key Structure"))
  (:`Pressed`
    (`GameplayStatics.ApplyDamage` self 10.0)))

(event `Key|Four`
  (params (Key :type "Key Structure"))
  (:`Pressed`
    (`GameplayStatics.ApplyDamage` self -20.0)))

(event `self.HealthComponent.OnDead`
  (`KismetSystemLibrary.PrintString` "DEAD!")
  (bind _asmain_char_bp (cast `/Game/MyBlueprints/Main_Char_BP` (`GameplayStatics.GetPlayerCharacter` 0)))
  (`self.DisableInput` _asmain_char_bp self)
  (set `self.bShowMouseCursor` true)
  (`SceneComponent.K2_AddLocalOffset` (`F_ProjectCharacter.CameraBoom` _asmain_char_bp) (-400.0 0.0 200.0) true true)
  (`|PlayMontage` (`Character.Mesh` _asmain_char_bp) "/Game/MyBlueprints/MyAnim/AM_Death.AM_Death"
    (:`then`
      (`|PlayMontage` (`/Game/MyBlueprints/Main_Char_BP.MESH_A_03` _asmain_char_bp) "/Game/MyBlueprints/MyAnim/AM_Death.AM_Death"
        (:`OnBlendOut`
          (`KismetSystemLibrary.Delay` 2.0)
          (`KismetSystemLibrary.QuitGame` null "Quit"))))))

(fn `UserConstructionScript`)