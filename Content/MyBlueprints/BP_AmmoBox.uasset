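; Ammo pickup that reloads the player character's weapon when touched.
; The construction script rolls a random AmmoAmount within a fixed range, and BeginPlay passes it to the WBP_Ammo widget on the Count component.
; Tick turns that widget toward the player camera.
; Overlapping Collision with the player character passes the amount to the Weapon's Reload, then destroys the box.
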(event `self.ReceiveTick`
  (params (DeltaSeconds :type "Float (single-precision)"))
  (bind _count (`self.Count`))
  ;[0 0 1] 3 Поворот виджета патронов
  (`SceneComponent.K2_SetWorldRotation` _count (`KismetMathLibrary.FindLookAtRotation` (`SceneComponent.K2_GetComponentLocation` _count) (`SceneComponent.K2_GetComponentLocation` (`PlayerCameraManager.TransformComponent` (`GameplayStatics.GetPlayerCameraManager` 0)))) false false))

(event `self.ReceiveBeginPlay`
  ;[1 1 1] Call Wiget AmmoCount
  (bind _aswbp_ammo (cast `/Game/MyUI/WBP_Ammo` (`WidgetComponent.GetUserWidgetObject` (`self.Count`))))
  (`/Game/MyUI/WBP_Ammo.SetAmmoCount` _aswbp_ammo (`self.AmmoAmount`)))

(event `self.Collision.OnComponentBeginOverlap`
  (params (OverlappedComponent :type "PrimitiveComponent Object Reference") (OtherActor :type "Actor Object Reference") (OtherComp :type "PrimitiveComponent Object Reference") (OtherBodyIndex :type Integer) (bFromSweep :type Boolean) (SweepResult :type "HitResult Structure (by ref)"))
  (bind _returnvalue (`GameplayStatics.GetPlayerCharacter` 0))
  (if (== OtherActor _returnvalue)
    (bind _asmain_char_bp (cast `/Game/MyBlueprints/Main_Char_BP` _returnvalue))
    (`/Game/MyBlueprints/Ka47_BP.Reload` (`/Game/MyBlueprints/Main_Char_BP.weapon` _asmain_char_bp) (`self.AmmoAmount`))
    (`self.K2_DestroyActor`)))

(fn `UserConstructionScript`
  (set `self.AmmoAmount` (`KismetMathLibrary.RandomIntegerInRange` 15 30)))