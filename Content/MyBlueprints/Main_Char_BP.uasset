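; Player character Blueprint with two switchable weapons, crouch, sprint and a HUD.
; BeginPlay creates the HUD, spawns Ka47 and KA_val attached to the hand mesh's weapon socket, and shows the second.
; Enhanced Input actions toggle weapon visibility and HUD, with a boolean routing shoot and reload to the active weapon.
; Debug-style keys quit the game or play death and hit-react montages on two meshes, disabling input during death.
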(event `EnhancedInput|/Game/ThirdPerson/Input/Actions/IA_Weapon2`
  (params (ActionValue :type Boolean) (ElapsedSeconds :type "Float (double-precision)") (TriggeredSeconds :type "Float (double-precision)") (InputAction :type "InputAction Object Reference" :default "/Game/ThirdPerson/Input/Actions/IA_Weapon2.IA_Weapon2"))
  (bind _weapon2 (`self.weapon2`))
  (:`Triggered`
    (`self.SetActorHiddenInGame` (`self.weapon1`) true)
    (`self.SetActorHiddenInGame` (`self.weapon2`) false)
    (`/Game/MyBlueprints/BP_KA_val.Equip` _weapon2)
    (set `self.weapon2` _weapon2)
    (set `self.whatweapon` false)
    (`/Game/MyUI/WBP_MainHUD.Weapon2Switch` (`self.MainHUD`))))

(event `EnhancedInput|/Game/ThirdPerson/Input/Actions/IA_Weapon1`
  (params (ActionValue :type Boolean) (ElapsedSeconds :type "Float (double-precision)") (TriggeredSeconds :type "Float (double-precision)") (InputAction :type "InputAction Object Reference" :default "/Game/ThirdPerson/Input/Actions/IA_Weapon1.IA_Weapon1"))
  (bind _weapon1 (`self.weapon1`))
  (:`Triggered`
    (`self.SetActorHiddenInGame` (`self.weapon2`) true)
    (`self.SetActorHiddenInGame` (`self.weapon1`) false)
    (`/Game/MyBlueprints/Ka47_BP.Equip` _weapon1)
    (set `self.weapon1` _weapon1)
    (set `self.whatweapon` true)
    (`/Game/MyUI/WBP_MainHUD.Weapon1Switch` (`self.MainHUD`))))

(event `self.ReceiveBeginPlay`
  (bind _weapon1 (`self.weapon1`))
  ;[1 1 1] Add_HUD
  (bind _returnvalue (`|CreateWidget` "/Game/MyUI/WBP_MainHUD.WBP_MainHUD_C"))
  (bind _output_get (set `self.MainHUD` _returnvalue))
  (`UserWidget.AddToViewport` _output_get 0)
  ;[1 1 1] Spawn Weapon
  (bind _returnvalue_2 (`|SpawnActorFromClass` "/Game/MyBlueprints/Ka47_BP.Ka47_BP_C" (`KismetMathLibrary.MakeTransform` (0.0 0.0 0.0)) "AlwaysSpawn" "MultiplyWithRoot" null null))
  (bind _output_get_2 (set `self.weapon1` _returnvalue_2))
  (`self.K2_AttachToComponent` _output_get_2 (`self.Mesh`) "Weapon_socket" "KeepRelative" "KeepRelative" "KeepRelative" true)
  ;[1 0 1] 2. Проверка подбора оружия персонажем?
  (`/Game/MyBlueprints/Ka47_BP.Equip` _weapon1)
  (`self.SetActorHiddenInGame` _weapon1 true)
  (bind _returnvalue_3 (`|SpawnActorFromClass` "/Game/MyBlueprints/BP_KA_val.BP_KA_val_C" (`KismetMathLibrary.MakeTransform` (0.0 0.0 0.0)) "AlwaysSpawn" "MultiplyWithRoot" null null))
  (bind _output_get_3 (set `self.weapon2` _returnvalue_3))
  (`self.K2_AttachToComponent` _output_get_3 (`self.Mesh`) "Weapon_socket" "KeepRelative" "KeepRelative" "KeepRelative" true)
  ;[1 0 1] 2. Проверка подбора оружия персонажем?
  (`/Game/MyBlueprints/BP_KA_val.Equip` (`self.weapon2`))
  (`/Game/MyUI/WBP_MainHUD.Weapon2Switch` (`self.MainHUD`)))

(event `Key|Q`
  (params (Key :type "Key Structure"))
  (:`Pressed`
    (`KismetSystemLibrary.QuitGame` null "Quit")))

(event `EnhancedInput|/Game/ThirdPerson/Input/Actions/IA_Shoot`
  (params (ActionValue :type Boolean) (ElapsedSeconds :type "Float (double-precision)") (TriggeredSeconds :type "Float (double-precision)") (InputAction :type "InputAction Object Reference" :default "/Game/ThirdPerson/Input/Actions/IA_Shoot.IA_Shoot"))
  (bind _weapon1 (`self.weapon1`))
  (bind _weapon2 (`self.weapon2`))
  (bind _whatweapon (`self.whatweapon`))
  ;[1 1 1] Shoot Meh
  (:`Started`
    (if _whatweapon
      (`/Game/MyBlueprints/Ka47_BP.StartShoot` _weapon1)
      (else
        (`/Game/MyBlueprints/BP_KA_val.StartShoot` _weapon2))))
  (:`Completed`
    (if _whatweapon
      (`/Game/MyBlueprints/Ka47_BP.StopShoot` _weapon1)
      (else
        (`/Game/MyBlueprints/BP_KA_val.StopShoot` _weapon2)))))

(event `EnhancedInput|/Game/ThirdPerson/Input/Actions/IA_Crouch`
  (params (ActionValue :type Boolean) (ElapsedSeconds :type "Float (double-precision)") (TriggeredSeconds :type "Float (double-precision)") (InputAction :type "InputAction Object Reference" :default "/Game/ThirdPerson/Input/Actions/IA_Crouch.IA_Crouch"))
  (:`Triggered`
    (`self.Crouch`))
  (:`Completed`
    (`self.UnCrouch`)))

(event `EnhancedInput|/Game/ThirdPerson/Input/Actions/IA_Reload`
  (params (ActionValue :type Boolean) (ElapsedSeconds :type "Float (double-precision)") (TriggeredSeconds :type "Float (double-precision)") (InputAction :type "InputAction Object Reference" :default "/Game/ThirdPerson/Input/Actions/IA_Reload.IA_Reload"))
  ;[1 1 1] Shoot Meh
  (:`Started`
    (if (`self.whatweapon`)
      (`/Game/MyBlueprints/Ka47_BP.Reload` (`self.weapon1`) 0)
      (else
        (`/Game/MyBlueprints/BP_KA_val.Reload` (`self.weapon2`) 0)))))

(event `EnhancedInput|/Game/ThirdPerson/Input/Actions/IA_Sprint`
  (params (ActionValue :type Boolean) (ElapsedSeconds :type "Float (double-precision)") (TriggeredSeconds :type "Float (double-precision)") (InputAction :type "InputAction Object Reference" :default "/Game/ThirdPerson/Input/Actions/IA_Sprint.IA_Sprint"))
  (bind _charactermovement (`self.CharacterMovement`))
  (:`Triggered`
    (set `CharacterMovementComponent.MaxWalkSpeed` 600.0 _charactermovement))
  (:`Completed`
    (set `CharacterMovementComponent.MaxWalkSpeed` 400.0 _charactermovement)))

(event `Key|K`
  (params (Key :type "Key Structure"))
  (:`Pressed`
    (`self.DisableInput` null)
    (`|PlayMontage` (`self.Mesh`) "/Game/MyBlueprints/MyAnim/AM_Death.AM_Death"
      (:`then`
        (`|PlayMontage` (`self.MESH_A_03`) "/Game/MyBlueprints/MyAnim/AM_Death.AM_Death"
          (:`OnCompleted`
            (`self.EnableInput` null)))))))

(event `Key|J`
  (params (Key :type "Key Structure"))
  (:`Pressed`
    (`|PlayMontage` (`self.Mesh`) "/Game/MyBlueprints/MyAnim/AM_HitReact.AM_HitReact"
      (:`then`
        (`|PlayMontage` (`self.MESH_A_03`) "/Game/MyBlueprints/MyAnim/AM_HitReact.AM_HitReact")))))

(fn `UserConstructionScript`)