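; Automatic hitscan rifle Blueprint (Ka47) that attaches to Main_Char_BP, tracks its ammo and updates that character's HUD.
; A looping timer fires line traces from the muzzle socket toward a distant point along the camera's forward vector.
; Shots spawn decals and sounds; blocking hits add an explosion effect, point damage and a short-lived FS_MasterField triggered at impact.
; Reload waits on a delay, adds ammo capped at the maximum, then signals completion.
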(event `Equip`
  (bind _asmain_char_bp (cast `/Game/MyBlueprints/Main_Char_BP` (`self.GetAttachParentActor`)))
  (set `self.Player` _asmain_char_bp)
  (`self.UpdateHud`))

(event `Reload`
  (params (Ammo :type Integer))
  (bind _returnvalue (+ Ammo (`self.Ammo`)))
  (`KismetSystemLibrary.PrintString` "RELOADING!")
  (`KismetSystemLibrary.RetriggerableDelay` 2.0) ; Reload time
  (if (> _returnvalue (`self.Ammo_Max`))
    (set `self.Ammo` (`self.Ammo_Max`))
    (else
      (set `self.Ammo` _returnvalue)))
  (`KismetSystemLibrary.PrintString` "RELOADED!")
  (`self.OnReloaded`)
  (`self.UpdateHud`))

(event `StopShoot`
  (`KismetSystemLibrary.K2_ClearAndInvalidateTimerHandle` (`self.ShootTimer`)))

(event `StartShoot`
  (bind _returnvalue (`KismetSystemLibrary.K2_SetTimerDelegate` (delegate `Shoot`) 0.1 true)) ; ShootSpeed
  (set `self.ShootTimer` _returnvalue)
  (`self.Shoot`))

(event `Shoot`
  (bind _returnvalue (`GameplayStatics.GetPlayerCameraManager` 0))
  (if (> (`self.Ammo`) 0)
    (`/Engine/EditorBlueprintResources/StandardMacros.DecrementInt` (`self.Ammo`)
      (:`  `
        (`self.UpdateHud`)
        ;[1 1 1] ShootVector
        (bind _outhit (`KismetSystemLibrary.LineTraceSingleForObjects` (`SceneComponent.K2_GetComponentLocation` (`self.Shoot_Soket`)) (+ (`PlayerCameraManager.GetCameraLocation` _returnvalue) (* (`self.GetActorForwardVector` _returnvalue) 10000)) (`|MakeArray` "ObjectTypeQuery1" "ObjectTypeQuery2" "ObjectTypeQuery3" :!type "EObjectTypeQuery Enum") false (`self.GetAttachedActors` true) "ForDuration" true (struct :`R` 1.0 :`A` 1.0) (struct :`G` 1.0 :`A` 1.0) 1.0))
        (bind (_bblockinghit _binitialoverlap _time _distance _location _impactpoint _normal _impactnormal _physmat _hitactor) (`GameplayStatics.BreakHitResult` _outhit))
        (bind _returnvalue_2 (`KismetMathLibrary.MakeRotFromX` _normal))
        (`GameplayStatics.SpawnDecalAtLocation` "/Game/MSPresets/M_MS_ImperfectionDecal_Material/M_MS_hall.M_MS_hall" (15.0 15.0 15.0) _location _returnvalue_2 20.0)
        (`GameplayStatics.SpawnSoundAtLocation` "/Engine/VREditor/Sounds/UI/Flashlight_Switch.Flashlight_Switch" (0.0 0.0 0.0) (struct) 1.0 1.0 0.0 null null)
        (if _bblockinghit
          (`GameplayStatics.SpawnEmitterAtLocation` "/Game/StarterContent/Particles/P_Explosion.P_Explosion" _location _returnvalue_2 (`KismetMathLibrary.Conv_DoubleToVector` 0.2) true "AutoRelease")
          (`GameplayStatics.ApplyPointDamage` _hitactor 10.0 _location _outhit)
          (bind _returnvalue_3 (`|SpawnActorFromClass` "/Engine/EditorResources/FieldNodes/FS_MasterField.FS_MasterField_C" (`KismetMathLibrary.MakeTransform` _location) "Undefined" "MultiplyWithRoot" null null))
          (set `/Engine/EditorResources/FieldNodes/FS_MasterField.ActivationType` "NewEnumerator4" _returnvalue_3)
          (`/Engine/EditorResources/FieldNodes/FS_MasterField.CE_Trigger` _returnvalue_3)
          (`KismetSystemLibrary.Delay` 0.02)
          (`self.K2_DestroyActor` _returnvalue_3))))
    (else
      (`KismetSystemLibrary.PrintString` "NO AMMO!")
      (`GameplayStatics.SpawnSoundAttached` "/Engine/VREditor/Sounds/UI/Scaling_Up.Scaling_Up" (`self.Shoot_Soket`) "None" (0.0 0.0 0.0) (struct) "KeepRelativeOffset" false 1.0 1.0 0.0 null null))))

(fn `GetAmmo`
  (params (Current :type Boolean))
  (returns (Result :type Integer))
  (if Current
    (return (`self.Ammo`))
    (else
      (return (`self.Ammo_Max`)))))

(fn `UpdateHud`
  (bind _player (`self.Player`))
  (`/Engine/EditorBlueprintResources/StandardMacros.IsValid` _player
    (:`Is Valid`
      (`/Game/MyUI/WBP_MainHUD.UpdateAmmoCount` (`/Game/MyBlueprints/Main_Char_BP.MainHUD` _player) (`self.Ammo`) (`self.Ammo_Max`)))))

(fn `UserConstructionScript`)